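; BP_MainGameInstance is the game instance that handles audio volume and music playback.
; Events set master, music and environment volume through sound mix class overrides, all writing to one shared Volume variable.
; A toggle reads that variable to mute or restore the master class at default volume.
; PlayMusic spawns a 2D sound that persists across level transitions and stores its reference.
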(event Custom|ChangeVolumeEnvironnement
  (params (NewVolume :type Float%20%28double-precision%29))
  (Audio|SetSoundMixClassOverride "/Game/Sound/SMIX_Environnement.SMIX_Environnement" "/Game/Sound/SC_Environnement.SC_Environnement" NewVolume 1.0 0.0 true)
  (Variables|Default|SetVolume NewVolume))

(event Custom|TurnOnOffVolume
  (if (== (Variables|Default|GetVolume) 0.0)
    (Audio|SetSoundMixClassOverride "/Game/Sound/SMIX_Master.SMIX_Master" "/Game/Sound/SC_Master.SC_Master" 1.0 1.0 0.0 true)
    (Variables|Default|SetVolume 1.0)
    (else
      (Audio|SetSoundMixClassOverride "/Game/Sound/SMIX_Master.SMIX_Master" "/Game/Sound/SC_Master.SC_Master" 0.0 1.0 0.0 true)
      (Variables|Default|SetVolume 0.0))))

(event Custom|ChangeVolumeMaster
  (params (NewVolume :type Float%20%28double-precision%29))
  (Audio|SetSoundMixClassOverride "/Game/Sound/SMIX_Master.SMIX_Master" "/Game/Sound/SC_Master.SC_Master" NewVolume 1.0 0.0 true)
  (Variables|Default|SetVolume NewVolume))

(event Custom|PlayMusic
  (params (Music :type Sound%20Wave%20Object%20Reference))
  (bind _returnvalue (Audio|SpawnSound2D Music 1.0 1.0 0.0 0 true))
  (Variables|Default|SetMusic _returnvalue))

(event Custom|ChangeVolumeMusic
  (params (NewVolume :type Float%20%28double-precision%29))
  (Audio|SetSoundMixClassOverride "/Game/Sound/SMIX_Music.SMIX_Music" "/Game/Sound/SC_Music.SC_Music" NewVolume 1.0 0.0 true)
  (Variables|Default|SetVolume NewVolume))