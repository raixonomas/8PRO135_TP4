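; BP_TargetSpawner is a spawn point that holds at most one shootable BP_Target at a time.
; SpawnTarget creates a target at its own location, yawed to face the player pawn on the horizontal plane, and hands it a back-reference.
; When TargetGetShot fires, it frees the slot and adds score through the BP_TargetSpawnerManager found at BeginPlay.
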(event Custom|SpawnTarget
  (bind _returnvalue (Transformation|GetActorTransform))
  (if (not (Variables|Default|GetHasATarget))
    (bind _returnvalue_2 (Game|SpawnActorfromClass "/Game/Blueprint/Target/BP_Target.BP_Target_C" (Math|Transform|MakeTransform (.location _returnvalue) (Math|Conversions|RotationFromXVector (Math|Vector|RotateVector (Math|Vector|Normalize (* (- (Transformation|GetActorLocation (Game|Player|GetPlayerPawn 0)) (Transformation|GetActorLocation)) "1.000000,1.000000,0.000000")) "0, 0, 0")) (.scale _returnvalue)) "Undefined" "MultiplyWithRoot" 0 0))
    (Variables|Default|SetHasATarget true)
    (Variables|/Game/Blueprint/Target/BP_Target.BP_Target_C|SetTargetSpawner _returnvalue_2 self)))

(event Custom|TargetGetShot
  (Variables|Default|SetHasATarget false)
  (Default|AddScore (Variables|Default|GetTargetSpawnerManager)))

(event EventBeginPlay
  (bind _returnvalue (Actor|GetActorOfClass "/Game/Blueprint/Target/BP_TargetSpawnerManager.BP_TargetSpawnerManager_C"))
  (Variables|Default|SetTargetSpawnerManager _returnvalue))

(fn ConstructionScript)