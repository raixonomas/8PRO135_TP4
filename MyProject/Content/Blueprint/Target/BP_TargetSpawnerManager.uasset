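; BP_TargetSpawnerManager runs the target minigame, timing target spawns and tracking the score.
; On BeginPlay it collects all BP_TargetSpawner actors and starts a looping timer that asks a random one to spawn a target.
; AddScore increments the score, updates the score widget as current over maximum, and opens the LVL_Race level once the maximum is reached.
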(event Custom|AskToSpawnTarget
  (Default|SpawnTarget (.OutItem (Utilities|Array|Random (Variables|Default|GetTargetSpawners)))))

(event Custom|AddScore
  (Variables|Default|SetScore (+ (Variables|Default|GetScore) 1))
  (Rendering|Components|TextRender|SetText (Variables|/Game/UI/FirstPersonShooter/W_Score.W_Score_C|Gettxt_Score (Variables|Default|GetScoreWidget)) (Utilities|Text|ToText(String) (Utilities|String|Append (Utilities|String|ToString(Text) (Utilities|Text|ToText(Integer) (Variables|Default|GetScore))) "/" (Utilities|String|ToString(Text) (Utilities|Text|ToText(Integer) (Variables|Default|GetMaxScore))))))
  (if (== (Variables|Default|GetScore) (Variables|Default|GetMaxScore))
    (Game|OpenLevel(byName) "LVL_Race")))

(event EventBeginPlay
  (bind _outactors (Actor|GetAllActorsOfClass "/Game/Blueprint/Target/BP_TargetSpawner.BP_TargetSpawner_C"))
  (Variables|Default|SetTargetSpawners _outactors)
  (Utilities|Time|SetTimerbyEvent (delegate Custom|AskToSpawnTarget) 1.0 true))

(fn ConstructionScript)